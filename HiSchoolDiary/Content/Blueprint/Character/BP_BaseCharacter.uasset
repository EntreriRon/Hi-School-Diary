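; Base combat character that builds its stats, mesh and camp-based material and collision from a data table row.
; Action events trigger AbilityStateMachine transitions or set gameplay tags, alongside ComboGraph attacks, grappling, sprinting and weapon pickup/throw.
; Damage drives hit montages, launch knockback and death, with timers handling falling, lying and get-up.
; Overlaps track nearby props and enemies; launch, montage and speed changes use paired client/server calls.
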(event Custom|Slomo
  (params (Duration :type Float%20%28double-precision%29) (TimeDilation :type Float%20%28double-precision%29))
  (Variables|Default|SetCustomTimeDilation TimeDilation)
  (Utilities|Time|SetTimerbyEvent (delegate Custom|TimeFreezeEnd) Duration))

(event Custom|OnKickedout
  (params (LaunchVelocity :type Vector) (bXYOverride :type Boolean) (bZOverride :type Boolean))
  (Character|LaunchCharacter LaunchVelocity bXYOverride bZOverride)
  (CallFunction|ServerKickedout LaunchVelocity bXYOverride bZOverride))

(event Custom|StopCurrentMontage
  (params (Blend%20Time :type Float%20%28single-precision%29))
  (bind _asbp_base_character_anim_inst (CallFunction|GetAnimInstacne))
  (bind _returnvalue (Animation|Montage|GetCurrentActiveMontage _asbp_base_character_anim_inst))
  (Utilities|IsValid _returnvalue
    (:Is%20Valid
      (if (== Blend%20Time 0.0)
        (Animation|Montage|MontageStop _asbp_base_character_anim_inst 0.0 _returnvalue)
        (else
          (Class|AnimInstance|MontageStopwithBlendOut _asbp_base_character_anim_inst (Utilities|Struct|MakeAlphaBlendArgs 0 Blend%20Time "ExpInOut") _returnvalue))))))

(event Custom|TimeFreezeEnd
  (Variables|Default|SetCustomTimeDilation 1.0))

(event Custom|ChangeBeenTargetedState
  (params (isTarget :type Boolean))
  (if isTarget
    (Rendering|SetVisibility (Variables|Default|GetBodyUI) true false)
    (else
      (Rendering|SetVisibility (Variables|Default|GetBodyUI) false false))))

(event Custom|ServerKickedout
  (params (LaunchVelocity :type Vector) (bXYOverride :type Boolean) (bZOverride :type Boolean))
  (Character|LaunchCharacter LaunchVelocity bXYOverride bZOverride))

(event Custom|OnTakeDamage_Front
  (params (Damage%20Data :type Struc%20Damage%20Data%20Structure))
  (bind (_caster _damagevalue _hiteffcttype _knockbackvelocity _knockupvelocity) (Utilities|Struct|BreakStruc_DamageData Damage%20Data))
  (bind _asbp_base_character_anim_inst (CallFunction|GetAnimInstacne))
  (bind _output_get (Variables|Default|SetCurrentHP (- (Variables|Default|GetCurrentHP) _damagevalue)))
  (Utilities|FlowControl|Sequence
    (:then_0
      (if (Tags|HasAnyAbilitiesTags (GameplayTags|MakeLiteralGameplayTagContainer "(GameplayTags=((TagName=\"Combat.Abilities.Falling\")))") true)
        (Ability|Animation|MontageJumptoSection (CallFunction|GetAnimInstacne) "FallingHit" (Variables|Assets|GetHitKnockoutAsset))
        (else
          (Tags|SetAbilitiesTags "(GameplayTags=((TagName=\"Combat.Status.Stun_Hit\")))")
          (Class|AnimInstance|MontageStopwithBlendOut _asbp_base_character_anim_inst (Utilities|Struct|MakeAlphaBlendArgs 0 0.2 "ExpOut") (Animation|Montage|GetCurrentActiveMontage _asbp_base_character_anim_inst))
          (Animation|Montage|PlayMontage (Variables|Character|GetMesh) (Utilities|Select :Index _hiteffcttype :NewEnumerator0 "/Game/Resource/Character/Lucy/Animations/Mont_Hit/Lucy_Hit_F_Inplace_Montage.Lucy_Hit_F_Inplace_Montage" :NewEnumerator1 "/Game/Resource/Character/Lucy/Animations/Mont_Hit/Lucy_Hit_FD_Inplace_Montage.Lucy_Hit_FD_Inplace_Montage" :NewEnumerator2 (Variables|Assets|GetHitKnockoutAsset) :NewEnumerator3 "/Game/Resource/Character/Common/Animation/Mont_hit_grapple.Mont_hit_grapple")
            (:OnBlendOut
              (Tags|SetAbilitiesTags "(GameplayTags=((TagName=\"Combat.Abilities.Idle\"),(TagName=\"Combat.Status\")))"))))))
    (:then_1
      (Variables|Default|SetKnockbackDirection (Math|Rotator|GetRotationXVector (Transformation|GetActorRotation _caster)))
      (if (not (Tags|HasAnyAbilitiesTags (GameplayTags|MakeLiteralGameplayTagContainer "(GameplayTags=((TagName=\"Combat.Abilities.Falling\")))") true))
        (CallFunction|OnKickedout (+ (* (Variables|Default|GetKnockbackDirection) (Math|Conversions|ToVector(Float) _knockbackvelocity)) (Math|Vector|MakeVector 0.0 0.0 _knockupvelocity)) false true :!label _label)
        (elif (Utilities|Enum|Equal(Enum) _hiteffcttype "NewEnumerator2")
          (goto _label)
          (else
            (CallFunction|OnKickedout (+ (* (Variables|Default|GetKnockbackDirection) "50.000000,0,0") "0,0,500.000000") true true)))))
    (:then_2
      (if (<= _output_get 0.0)
        (Utilities|FlowControl|DoOnce false :!label _label_2
          (:Completed
            (Default|CallOnDying self)))
        (else
          (goto _label_2 Reset))))))

(event EventBeginPlay
  (EventDispatchers|BindEventtoOnTakeDamage (Variables|Default|GetDamageComponent) (delegate Custom|OnTakeDamage_Front))
  (Variables|/Game/Blueprint/UI/WorldWidget/BP_WUI_Head.BP_WUI_Head_C|SetParentCharacter (CallFunction|GetHeadUI) self))

(event OnComponentBeginOverlap(CapsuleComponent)
  (params (OverlappedComponent :type Primitive%20Component%20Object%20Reference) (OtherActor :type Actor%20Object%20Reference) (OtherComp :type Primitive%20Component%20Object%20Reference) (OtherBodyIndex :type Integer) (bFromSweep :type Boolean) (SweepResult :type Hit%20Result%20Structure%20%28by%20ref%29))
  ;[1 1 1] Props register
  (bind _asbp_base_props (Utilities|Casting|CastToBP_BaseProps OtherActor))
  (Utilities|Array|AddUnique (Variables|Default|GetPropsAround) _asbp_base_props)
  (Game|BindEventtoOnDestroyed _asbp_base_props (delegate Custom|PropsAroundDestory)))

(event OnComponentEndOverlap(CapsuleComponent)
  (params (OverlappedComponent :type Primitive%20Component%20Object%20Reference) (OtherActor :type Actor%20Object%20Reference) (OtherComp :type Primitive%20Component%20Object%20Reference) (OtherBodyIndex :type Integer))
  ;[1 1 1] Props register
  (bind _asbp_base_props (Utilities|Casting|CastToBP_BaseProps OtherActor))
  (CallFunction|PropsAroundDestory _asbp_base_props))

(event OnComponentBeginOverlap(EnemyDetector)
  (params (OverlappedComponent :type Primitive%20Component%20Object%20Reference) (OtherActor :type Actor%20Object%20Reference) (OtherComp :type Primitive%20Component%20Object%20Reference) (OtherBodyIndex :type Integer) (bFromSweep :type Boolean) (SweepResult :type Hit%20Result%20Structure%20%28by%20ref%29))
  (bind _asbp_base_character (Utilities|Casting|CastToBP_BaseCharacter OtherActor))
  (if (!= _asbp_base_character self)
    (if (Utilities|Enum|Equal(Enum) (Variables|BP_BaseCharacter_C|GetCamp _asbp_base_character) "NewEnumerator1")
      (Utilities|Array|AddUnique (Variables|Default|GetNearbyEnemys) _asbp_base_character))))

(event OnComponentEndOverlap(EnemyDetector)
  (params (OverlappedComponent :type Primitive%20Component%20Object%20Reference) (OtherActor :type Actor%20Object%20Reference) (OtherComp :type Primitive%20Component%20Object%20Reference) (OtherBodyIndex :type Integer))
  (bind _asbp_base_character (Utilities|Casting|CastToBP_BaseCharacter OtherActor))
  (if (!= _asbp_base_character self)
    (if (Utilities|Enum|Equal(Enum) (Variables|BP_BaseCharacter_C|GetCamp _asbp_base_character) "NewEnumerator1")
      (Utilities|Array|RemoveItem (Variables|Default|GetNearbyEnemys) _asbp_base_character))))

(event Custom|ActionMove
  (params (MoveDirection :type Vector%202D%20Structure) (MoveScale :type Float%20%28single-precision%29))
  ;[0.5401 0.8997 1] Movement
  ;;[0.5665 0.7455 1] Idle/Move
  (Variables|Default|SetMoveSpeed MoveScale)
  (Default|TriggerTransition (Variables|Default|GetAbilityStateMachine) "(TagName=\"Combat.Abilities.Move\")"))

(event Custom|SyncAbortRecovery
  (params (Blend%20Time :type Float%20%28single-precision%29))
  (bind _self self)
  (bind _returnvalue (Ability|GetAbilitySystemComponent _self))
  ;[0 0 0] Recovery
  (bind _outabilityhandles (Class|AbilitySystemComponent|GetAllAbilities _returnvalue))
  (for _array_element _outabilityhandles
    (Ability|CancelAbility (.ReturnValue (Ability|GameplayAbility|GetGameplayAbilityfromSpecHandle _returnvalue _array_element)))))

(event Custom|LyingFinished
  ;[1 1 1] Lying
  (Animation|Montage|PlayMontage (Variables|Character|GetMesh) "/Game/Resource/Character/Lucy/Animations/Mont_Hit/Lucy_Hit_Up_GetUp_Inplace_Montage.Lucy_Hit_Up_GetUp_Inplace_Montage"
    (:then
      (Tags|SetAbilitiesTags "(GameplayTags=((TagName=\"Combat.Abilities.Idle\")))"))
    (:OnBlendOut
      (if (Tags|HasAnyAbilitiesTags (GameplayTags|MakeLiteralGameplayTagContainer "(GameplayTags=((TagName=\"Combat.Abilities.Dying\")))") true)
        (Actor|DestroyActor)))))

(event Custom|ActionSprint
  (params (Sprint :type Boolean))
  ;[0.5401 0.8997 1] Movement
  ;;[0.3216 0.9602 1] Sprint
  (if Sprint
    (Variables|Default|SetinSprint Sprint)
    (bind _alpha (Timeline|TL%20Sprint Play)
      (:Update
        (CallFunction|ChangeMoveSpeedServer (Math|Float|Lerp 4e+02 6e+02 _alpha)))
      (:Finished
        (Variables|Default|SetinSprint Sprint)))
    (else
      (Timeline|TL%20Sprint Reverse))))

(event Custom|Action_PickupNearestWeapon
  ;[1 0.9109 0.1354] Weapon
  (if (not (.Equiped (CallFunction|IsEquipedwithWeapon)))
    (bind _nearestprop (CallFunction|FindNearestWeapon))
    (Utilities|IsValid _nearestprop
      (:Is%20Valid
        (CallFunction|PickupWeapon _nearestprop)))))

(event Custom|ActionAttack
  ;[1 0.2083 0.2182] Attack
  (Default|TriggerTransition (Variables|Default|GetAbilityStateMachine) "(TagName=\"Combat.Abilities.Attack\")"))

(event Custom|ActionFalling
  ;[1 1 1] Falling
  (Tags|SetAbilitiesTags "(GameplayTags=((TagName=\"Combat.Abilities.Falling\")))")
  (CallFunction|UpdateFallingState)
  (bind _returnvalue (Utilities|Time|SetTimerbyEvent (delegate Custom|UpdateFallingState) 0.016 true))
  (Variables|Default|SetFallingTimer _returnvalue)
  (Collision|SetCollisionResponsetoChannel (Variables|Collision|GetCapsuleComponent) "ECC_Pawn" "ECR_Overlap"))

(event Custom|UpdateFallingState
  ;[1 1 1] Falling
  (if (not (AI|Components|NavMovement|IsFalling (Variables|Character|GetCharacterMovement)))
    (Animation|Montage|PlayMontage (Variables|Character|GetMesh) (Variables|Assets|GetHitKnockoutAsset) 1.0 0.0 "FallingFinshed"
      (:then
        (Utilities|Time|ClearandInvalidateTimerbyHandle (Variables|Default|GetFallingTimer))
        (Tags|SetAbilitiesTags "(GameplayTags=((TagName=\"Combat.Abilities.Lying\")))")
        (Collision|SetCollisionResponsetoChannel (Variables|Collision|GetCapsuleComponent) "ECC_Pawn" "ECR_Block")))))

(event Custom|Idle
  ;[0.5401 0.8997 1] Movement
  ;;[0.5665 0.7455 1] Idle/Move
  (Default|TriggerTransition (Variables|Default|GetAbilityStateMachine) "(TagName=\"Combat.Abilities.Idle\")"))

(event Custom|PickupWeapon
  (params (Weapon :type BP%20Base%20Weapon%20Object%20Reference))
  ;[1 0.9109 0.1354] Weapon
  (Default|PickupIt Weapon self)
  (Variables|Default|SetEquippedWeapon Weapon))

(event Custom|PlayMontage_Server
  (params (MontageToPlay :type Anim%20Montage%20Object%20Reference))
  (Animation|Montage|PlayMontage (Variables|Character|GetMesh) MontageToPlay))

(event Custom|ActionRecovery
  ;[0 0 0] Recovery
  (Default|TriggerTransition (Variables|Default|GetAbilityStateMachine) "(TagName=\"Combat.Abilities.AttackRecovery\")"))

(event Custom|PlayMontage
  (params (MontageToPlay :type Anim%20Montage%20Object%20Reference))
  (CallFunction|PlayMontageClient MontageToPlay)
  (CallFunction|PlayMontageServer MontageToPlay))

(event Custom|Action_Die
  (bind _mont_die_assets (Variables|Assets|GetMont_Die_Assets))
  (Variables|Default|SetbDead true)
  (Tags|AddAbilitiesTag "(TagName=\"Combat.Abilities.Dying\")")
  (if (not (Tags|HasAnyAbilitiesTags (GameplayTags|MakeLiteralGameplayTagContainer "(GameplayTags=((TagName=\"Combat.Abilities.Lying\"),(TagName=\"Combat.Abilities.Falling\")))") true))
    (CallFunction|PlayMontage (Utilities|Array|Get(acopy) _mont_die_assets (Math|Random|RandomIntegerinRange 0 (- (Utilities|Array|Length _mont_die_assets) 0))))))

(event Custom|ActionGrab
  (bind _grabsuccess (Default|TryGrab (Variables|Default|GetGrappleComponent)))
  (if _grabsuccess
    (Tags|SetAbilitiesTags "(GameplayTags=((TagName=\"Combat.Abilities.Grapple\")))")))

(event Custom|GrabAttack
  (Default|GrabAttack (Variables|Default|GetGrappleComponent)))

(event Custom|PlayMontage_Client
  (params (MontageToPlay :type Anim%20Montage%20Object%20Reference))
  (Animation|Montage|PlayMontage (Variables|Character|GetMesh) MontageToPlay))

(event Custom|PropsAroundDestory
  (params (DestroyedActor :type Actor%20Object%20Reference))
  (bind _propsaround (Variables|Default|GetPropsAround))
  ;[1 1 1] Props register
  (bind _asbp_base_props (Utilities|Casting|CastToBP_BaseProps DestroyedActor))
  (if (Utilities|Array|ContainsItem _propsaround _asbp_base_props)
    (Utilities|Array|RemoveItem _propsaround _asbp_base_props)))

(event Custom|ChangeMoveSpeed_Server
  (params (Max%20Walk%20Speed :type Float%20%28single-precision%29))
  ;[0.5401 0.8997 1] Movement
  ;;[0.3216 0.9602 1] Sprint
  (bind _output_get (Variables|/Script/Engine.CharacterMovementComponent|SetMaxWalkSpeed (Variables|Character|GetCharacterMovement) Max%20Walk%20Speed))
  (CallFunction|ChangeMoveSpeedClient _output_get))

(event Custom|ThrowWeapon
  ;[1 0.9109 0.1354] Weapon
  (if (.Equiped (CallFunction|IsEquipedwithWeapon))
    (CallFunction|PlayMontage "/Game/Resource/Item/Weapon/Mont_Weapon_Throw.Mont_Weapon_Throw")))

(event Custom|ChangeMoveSpeed_Client
  (params (Max%20Walk%20Speed :type Float%20%28single-precision%29))
  ;[0.5401 0.8997 1] Movement
  ;;[0.3216 0.9602 1] Sprint
  (Variables|/Script/Engine.CharacterMovementComponent|SetMaxWalkSpeed (Variables|Character|GetCharacterMovement) Max%20Walk%20Speed))

(event Custom|ActionDash
  ;[0.5401 0.8997 1] Movement
  ;;[0.06447 0.4112 1] Dash/Dodge
  (Default|TriggerTransition (Variables|Default|GetAbilityStateMachine) "(TagName=\"Combat.Abilities.Dash\")"))

(event Custom|WeaponLaunch
  (bind (_equiped _weapon) (CallFunction|IsEquipedwithWeapon))
  ;[1 0.9109 0.1354] Weapon
  (if _equiped
    (Default|LaunchWeapon _weapon (Math|Rotator|GetRotationXVector (Transformation|GetActorRotation)) self)
    (Variables|Default|SetEquippedWeapon 0)))

(event Custom|ComboStart
  (params (ComboGraph :type Combo%20Graph%20Object%20Reference))
  ;[1 0.2083 0.2182] Attack
  ;;[0.2157 1 0.2198] ComboGraph
  (if (not (Variables|Default|GetHasComboGraphActived))
    (bind _output_get (Variables|Default|SetCurrentComboGraph ComboGraph))
    (bind _asynctaskproxy (|TaskStartComboGraph (Variables|Default|GetComboGraphSystem) _output_get "/Game/Resource/Data/InputAction/InputAction_LightAttack.InputAction_LightAttack" true)
      (:OnActivationSuccess
        (Variables|Default|SetHasComboGraphActived true)
        (Variables|Default|SetCurrentComboAsyncTask _asynctaskproxy))
      (:OnActivationFailed
        (CallFunction|ActionRecovery))
      (:OnGraphEnd
        (Variables|Default|SetHasComboGraphActived false)
        (Variables|Default|SetCurrentComboAsyncTask 0)
        (Variables|Default|SetCurrentComboGraph 0)))))

(event Custom|ComboInputAction
  (params (Optional%20Object :type Object%20Object%20Reference))
  ;[1 0.2083 0.2182] Attack
  ;;[0.2157 1 0.2198] ComboGraph
  (Class|ComboGraphGameplayTasksComponent|SendGameplayEventReplicated (Variables|Default|GetComboGraphSystem) "(TagName=\"Event.ComboGraph.Input\")" (Utilities|Struct|MakeGameplayEventData "(TagName=\"Event.ComboGraph.Input\")" 0 0 Optional%20Object)))

(event Custom|AbortRecoveryServer
  (params (Blend%20Time :type Float%20%28single-precision%29))
  (bind _self self)
  (bind _returnvalue (Ability|GetAbilitySystemComponent _self))
  ;[0 0 0] Recovery
  (bind _outabilityhandles (Class|AbilitySystemComponent|GetAllAbilities _returnvalue))
  (for _array_element _outabilityhandles
    (Ability|CancelAbility (.ReturnValue (Ability|GameplayAbility|GetGameplayAbilityfromSpecHandle _returnvalue _array_element)))))

(event Custom|ActionLying
  ;[1 1 1] Lying
  (Tags|SetAbilitiesTags "(GameplayTags=((TagName=\"Combat.Abilities.Lying\")))")
  (Utilities|Time|SetTimerbyEvent (delegate Custom|LyingFinished) 1.0))

(event Custom|AbortRecovery
  (params (Blend%20Time :type Float%20%28single-precision%29))
  ;[0 0 0] Recovery
  (CallFunction|SyncAbortRecovery Blend%20Time)
  (CallFunction|AbortRecoveryServer Blend%20Time))

(event EventTick
  (params (DeltaSeconds :type Float%20%28single-precision%29))
  ;[1 0 0] Tick
  (Variables|Default|SetCurr%20State (Variables|/Game/Blueprint/Gameplay/Component/BPC_CharacterStateMachine.BPC_CharacterStateMachine_C|GetCurrStateObj (Variables|Default|GetAbilityStateMachine))))

(fn ConstructionScript
  (CallFunction|InitData)
  (CallFunction|AssembleAvatar)
  (CallFunction|InitCamp))

(fn GetAnimInstacne
  (bind _asbp_base_character_anim_inst (Utilities|Casting|CastToBP_BaseCharacterAnimInst (Components|SkeletalMesh|GetAnimInstance (Variables|Character|GetMesh))))
  (return _asbp_base_character_anim_inst))

(fn AssembleAvatar
  (bind _returnvalue (Utilities|LoadAssetBlocking (Utilities|Struct|BreakStruc_ChrAvatarData (Utilities|Struct|BreakStruc_ChrBaseData (Variables|Data|GetData)))))
  (bind _asskeletal_mesh (Utilities|Casting|CastToSkeletalMesh _returnvalue))
  (Class|SkinnedMeshComponent|SetSkeletalMesh (Variables|Character|GetMesh) _asskeletal_mesh true))

(fn InitCamp
  (bind _camp (Variables|Default|GetCamp))
  (Rendering|Material|SetMaterial (Variables|Character|GetMesh) 0 (Utilities|Select :Index _camp :NewEnumerator0 "/Game/Resource/Character/Common/Material/MI_Player_Female_Body.MI_Player_Female_Body" :NewEnumerator1 "/Game/Resource/Character/Common/Material/MI_Enemy_Female_Body.MI_Enemy_Female_Body" :NewEnumerator2 "/Game/Resource/Character/Common/Material/MI_Female_Body.MI_Female_Body"))
  (Collision|SetCollisionResponsetoChannel (Variables|Collision|GetCapsuleComponent) "ECC_GameTraceChannel1" (Utilities|Select :Index _camp :NewEnumerator0 "ECR_Ignore" :NewEnumerator1 "ECR_Overlap" :NewEnumerator2 "ECR_Ignore")))

(fn InitData
  (Utilities|FlowControl|Sequence
    (:then_0
      (bind _returnvalue (Utilities|GetDataTableRow "/Game/Data/DT_Character.DT_Character" (Utilities|String|StringToName (Utilities|String|ToString(Integer) (Variables|Data|GetCfgid))))
        (:then
          (Variables|Data|SetData _returnvalue))
        (:RowNotFound
          (bind _returnvalue_2 (Utilities|GetDataTableRow "/Game/Data/DT_Character.DT_Character" "10010")
            (:then
              (Variables|Data|SetData _returnvalue_2))))))
    (:then_1
      (Variables|Default|SetCurrentHP (CallFunction|GetMaxHP)))))

(fn GetMaxHP
  (return (Utilities|Struct|BreakStruc_ChrBattleData (.BattleData (Utilities|Struct|BreakStruc_ChrBaseData (Variables|Data|GetData))))))

(fn GetHeadUI
  (bind _asbp_wui_head (Utilities|Casting|CastToBP_WUI_Head (UserInterface|GetWidget (Variables|Default|GetHeadUI))))
  (return _asbp_wui_head))

(fn GetOwnerCharacter
  (return 0))

(fn CanMove
  (return (Tags|HasAnyAbilitiesTags (GameplayTags|MakeLiteralGameplayTagContainer "(GameplayTags=((TagName=\"Combat.Abilities.Move\"),(TagName=\"Combat.Abilities.Idle\"),(TagName=\"Combat.Abilities.AttackRecovery\")))") true)))

(fn FindNearestProps
  (params (Props :type Array%20of%20BP%20Base%20Props%20Object%20References))
  (bind _returnvalue (Transformation|GetActorLocation))
  (for _array_element Props
    (Utilities|IsValid (LocalVariables|GetL_NearestProp)
      (:Is%20Valid
        (if (< (Math|Vector|Distance(Vector) (Transformation|GetActorLocation _array_element) _returnvalue) (Math|Vector|Distance(Vector) (Transformation|GetActorLocation (LocalVariables|GetL_NearestProp)) _returnvalue))
          (LocalVariables|SetL_NearestProp _array_element)))
      (:Is%20Not%20Valid
        (LocalVariables|SetL_NearestProp _array_element))))
  (return (LocalVariables|GetL_NearestProp)))

(fn FindNearestWeapon
  (bind _returnvalue (Transformation|GetActorLocation))
  (for _array_element (Variables|Default|GetPropsAround)
    (bind _asbp_base_weapon (Utilities|Casting|CastToBP_BaseWeapon _array_element))
    (if (Variables|/Game/Blueprint/Gameplay/Interactive/Weapon/BP_BaseWeapon.BP_BaseWeapon_C|GetcanPickup _asbp_base_weapon)
      (Utilities|IsValid (LocalVariables|GetL_NearestProp)
        (:Is%20Valid
          (if (< (Math|Vector|Distance(Vector) (Transformation|GetActorLocation _asbp_base_weapon) _returnvalue) (Math|Vector|Distance(Vector) (Transformation|GetActorLocation (LocalVariables|GetL_NearestProp)) _returnvalue))
            (LocalVariables|SetL_NearestProp _asbp_base_weapon)))
        (:Is%20Not%20Valid
          (LocalVariables|SetL_NearestProp _asbp_base_weapon)))))
  (return (LocalVariables|GetL_NearestProp)))

(fn IsEquipedwithWeapon
  (bind _equippedweapon (Variables|Default|GetEquippedWeapon))
  (return (Utilities|IsValid _equippedweapon) _equippedweapon))

(fn SetAbilitiesTags
  (params (Tags :type Gameplay%20Tag%20Container%20Structure))
  (if (not (GameplayTags|HasAnyTags (Variables|Default|GetAbilityTags) Tags true))
    (for _array_element (GameplayTags|BreakGameplayTagContainer (Variables|Default|GetLastAbilityTags))
      (GameplayTags|RemoveGameplayTag (Variables|Default|GetAbilityTags) _array_element :!class /Script/GameplayTags.BlueprintGameplayTagLibrary))
    (bind _output_get (Variables|Default|SetLastAbilityTags Tags))
    (for _array_element_2 (GameplayTags|BreakGameplayTagContainer _output_get)
      (Tags|AddAbilitiesTag _array_element_2))
    (Default|CallOnTagsChanged self)))

(fn HasAnyAbilitiesTags
  (params (Tags :type Gameplay%20Tag%20Container%20Structure%20%28by%20ref%29) (bExactMatch :type Boolean))
  (return (GameplayTags|HasAnyTags (Variables|Default|GetAbilityTags) Tags bExactMatch)))

(fn AddAbilitiesTag
  (params (Tag :type Gameplay%20Tag%20Structure))
  (GameplayTags|AddGameplayTag (Variables|Default|GetAbilityTags) Tag :!class /Script/GameplayTags.BlueprintGameplayTagLibrary)
  (CallFunction|CustomPrintString "Combo" (Utilities|String|Append "NewTags:" (Utilities|String|ToString(Name) (GameplayTags|GetTagName Tag))) true true false))

(fn RemoveAbilitiesTag
  (params (Tag :type Gameplay%20Tag%20Structure))
  (GameplayTags|RemoveGameplayTag (Variables|Default|GetAbilityTags) Tag :!class /Script/GameplayTags.BlueprintGameplayTagLibrary))