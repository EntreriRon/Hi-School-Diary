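; BP_BasePlayer is a base player character Blueprint that adds enemy-detector debugging and attack-facing correction.
; DebugEnemyDetector toggles the detector sphere's visibility and spawns or destroys an attached particle scaled to its radius.
; Tick rotates that particle toward the player controller's transformed desired move direction.
; FixAttackRotation_1 snaps control rotation to the same direction, while a leftover enemy-list sequence is never run.
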(event Custom|DebugEnemyDetector
  (params (on :type Boolean))
  (if on
    (bind _returnvalue (Effects|SpawnEmitterAttached "/Game/Resource/VFX/Debug/P_FX_DebugEnemyDetector.P_FX_DebugEnemyDetector" (Variables|Default|GetCapsuleComponent) "None" "0, 0,-88.000000" "0, 0, 0" (Math|Conversions|ToVector(Float) (/ (Variables|/Script/Engine.SphereComponent|GetSphereRadius (Variables|Default|GetEnemyDetector)) 5e+01)) "KeepRelativeOffset" false))
    (bind _output_get (Variables|Default|SetDebugDetectorParticle _returnvalue))
    (Effects|Components|ParticleSystem|SetFloatParameter _output_get "Angle" 9e+01)
    (Development|SetHiddeninGame (Variables|Default|GetEnemyDetector) false false)
    (else
      (Utilities|IsValid (Variables|Default|GetDebugDetectorParticle)
        (:Is%20Valid
          (Components|DestroyComponent (Variables|Default|GetDebugDetectorParticle))
          (Development|SetHiddeninGame (Variables|Default|GetEnemyDetector) true false))))))

(event Custom|FixAttackRotation_1
  (bind _controller (CallFunction|GetGAPlayerController))
  (Pawn|SetControlRotation _controller (Default|TransformDesiredMoveRotation _controller (Variables|/Game/Blueprint/Gameplay/BP_BasePlayerController.BP_BasePlayerController_C|GetMove%20Direction _controller))))

(event EventTick
  (params (DeltaSeconds :type Float%20%28single-precision%29))
  (bind _controller (CallFunction|GetGAPlayerController))
  (bind _debugdetectorparticle (Variables|Default|GetDebugDetectorParticle))
  (|CallParentFunction DeltaSeconds)
  (Utilities|IsValid _debugdetectorparticle
    (:Is%20Valid
      (Transformation|SetWorldRotation _debugdetectorparticle (Default|TransformDesiredMoveRotation _controller (Variables|/Game/Blueprint/Gameplay/BP_BasePlayerController.BP_BasePlayerController_C|GetMove%20Direction _controller)) false false))))

(fn ConstructionScript
  (|CallParentFunction))