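; BPFunc_Common is a shared function library of global helpers for the HischoolDiary game.
; Typed getters cast to the project's game mode, game state, game instance, first player controller, its pawn, base HUD and network indicator.
; Utilities check online or server-player status, toggle an actor's visibility, collision and tick, and show info text to one player or all controllers.
; CustomPrintString prints only log types listed in the HUD's GM panel.
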(fn GetGAGameMode
  (bind _asbp_hischool_diary_game_mode (Utilities|Casting|CastToBP_HischoolDiaryGameMode (Game|GetGameMode (LocalVariables|Get__WorldContext))))
  (return _asbp_hischool_diary_game_mode))

(fn GetGAPlayerController
  (bind _asbp_base_player_controller (Utilities|Casting|CastToBP_BasePlayerController (Game|GetPlayerController 0)))
  (return _asbp_base_player_controller))

(fn GetPlayerBaseHUD
  (params (player_controller :type BP%20Base%20Player%20Controller%20Object%20Reference))
  (if (Utilities|IsValid player_controller)
    (LocalVariables|Settemp_controller player_controller)
    (else
      (bind _asbp_base_player_controller (Utilities|Casting|CastToBP_BasePlayerController (Game|GetPlayerController 0)))
      (LocalVariables|Settemp_controller _asbp_base_player_controller)))
  (bind _asbp_hud_base (Utilities|Casting|CastToBP_HUD_Base (HUD|GetHUD (LocalVariables|Gettemp_controller))))
  (return (Variables|/Game/Blueprint/UI/BP_HUD_Base.BP_HUD_Base_C|GetBaseHUD _asbp_hud_base)))

(fn GetControlledCharacter
  (bind _asbp_base_player (Utilities|Casting|CastToBP_BasePlayer (Pawn|GetControlledPawn (CallFunction|GetGAPlayerController))))
  (return _asbp_base_player))

(fn CustomPrintString
  (params (Type :type Name :default "Default") (InString :type String) (bPrintToScreen :type Boolean) (bPrintToLog :type Boolean) (OutputTimeSec :type Boolean))
  (bind _basehud (CallFunction|GetPlayerBaseHUD))
  (Utilities|IsValid _basehud
    (:Is%20Valid
      (LocalVariables|SetL_StringData (Utilities|Struct|MakeStruc_PrintString InString bPrintToScreen bPrintToLog))
      (if (Utilities|Array|ContainsItem (Variables|/Game/Blueprint/UI/BP_UI_GMPanel.BP_UI_GMPanel_C|GetLogTypeNames (Variables|/Game/Blueprint/UI/BP_UI_BaseHUD.BP_UI_BaseHUD_C|GetBP_UI_GMPanel _basehud)) Type)
        (Development|PrintString 0 (Utilities|String|SelectString (Utilities|String|Append (.InString (Utilities|Struct|BreakStruc_PrintString (LocalVariables|GetL_StringData))) "          :" (Utilities|String|ToString(Float) (Utilities|Time|GetTimeSeconds))) (.InString (Utilities|Struct|BreakStruc_PrintString (LocalVariables|GetL_StringData))) OutputTimeSec) (.PrinttoScreen (Utilities|Struct|BreakStruc_PrintString (LocalVariables|GetL_StringData))) (.PrinttoLog (Utilities|Struct|BreakStruc_PrintString (LocalVariables|GetL_StringData))))))))

(fn IsOnline
  (bind _asbp_hsd_game_instance (Utilities|Casting|CastToBP_HSD_GameInstance (Game|GetGameInstance)))
  (return (Variables|/Game/Blueprint/Gameplay/BP_HSD_GameInstance.BP_HSD_GameInstance_C|Getis_online _asbp_hsd_game_instance)))

(fn GetGAGameInstance
  (bind _asbp_hsd_game_instance (Utilities|Casting|CastToBP_HSD_GameInstance (Game|GetGameInstance)))
  (return _asbp_hsd_game_instance))

(fn GetNetworkIndicator
  (bind _asbp_ui_network (Utilities|Casting|CastToBP_UI_Network (UserInterface|GetWidget (Variables|/Game/Blueprint/Gameplay/BP_BasePlayerController.BP_BasePlayerController_C|GetNetworkIndicator (CallFunction|GetGAPlayerController)))))
  (return _asbp_ui_network))

(fn EnableActor
  (params (actor :type Actor%20Object%20Reference) (enabled :type Boolean))
  (Utilities|FlowControl|Sequence
    (:then_0
      (Rendering|SetActorHiddenInGame actor (not enabled)))
    (:then_1
      (Collision|SetActorEnableCollision actor enabled))
    (:then_2
      (Actor|Tick|SetActorTickEnabled actor enabled))))

(fn GetGAGameState
  (bind _asbp_hsd_game_state (Utilities|Casting|CastToBP_HSD_GameState (Game|GetGameState)))
  (return _asbp_hsd_game_state))

(fn IsServerPlayer
  (params (controller :type Controller%20Object%20Reference))
  (return (and (Pawn|IsLocalPlayerController controller) (Networking|IsServer))))

(fn ShowInfotoPlayer
  (params (player :type BP%20Base%20Player%20Controller%20Object%20Reference) (text :type String) (time :type Float%20%28double-precision%29))
  (if (Utilities|IsValid player)
    (Default|ShowInfoText player text time)
    (else
      (bind _outactors (Actor|GetAllActorsOfClass 0 "/Game/Blueprint/Gameplay/BP_BasePlayerController.BP_BasePlayerController_C"))
      (for _array_element _outactors
        (Default|ShowInfoText _array_element text time)))))