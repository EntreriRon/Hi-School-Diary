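; Player lock-on component that picks the nearest enemy inside a sector and flags it as targeted.
; It gathers opposing-camp characters overlapping the owner's EnemyDetector, skipping those tagged Lying.
; While the player has move input, a dot-product test against a zero-rotation forward vector filters candidates, then 2D distance selects the nearest.
; Tag-change bindings drop enemies that become Lying and rerun the targeting.
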(event Custom|ClearEnemys
  (Utilities|Array|Clear (Variables|Default|GetPredetectEnemys))
  (Variables|Default|SetNearestEnemy 0))

(event Custom|TryLockonTarget
  (bind _insectorenemy (Variables|Default|GetInSectorEnemy))
  (bind _insectorenemy_2 (Variables|Default|GetInSectorEnemy))
  (bind _nearestenemy (Variables|Default|GetNearestEnemy))
  (CallFunction|Init)
  (if (> (Variables|/Game/Blueprint/Gameplay/BP_BasePlayerController.BP_BasePlayerController_C|GetMove%20Scale (CallFunction|GetGAPlayerController)) 0.0)
    (if (> (Utilities|Array|Length (Variables|Default|GetPredetectEnemys)) 0)
      (for _array_element (Variables|Default|GetPredetectEnemys)
        (if (CallFunction|IsinSectorArea (Math|Vector|GetForwardVector "0, 0, 0") (Variables|Default|GetSectorAngle) _array_element)
          (Utilities|Array|AddUnique (Variables|Default|GetInSectorEnemy) _array_element)
          (elif (Utilities|Array|ContainsItem _insectorenemy _array_element)
            (Utilities|Array|RemoveItem _insectorenemy _array_element)
            (CallFunction|ChangeNearestEnemy))))
      (if (> (Utilities|Array|Length _insectorenemy_2) 0)
        (for _array_element_2 _insectorenemy_2
          (Utilities|IsValid _nearestenemy
            (:Is%20Valid
              (if (< (CallFunction|GetDisBetweenTargettoOwner _array_element_2) (CallFunction|GetDisBetweenTargettoOwner _nearestenemy))
                (CallFunction|ChangeNearestEnemy _array_element_2)))
            (:Is%20Not%20Valid
              (CallFunction|ChangeNearestEnemy _array_element_2))))
        (else
          (Utilities|IsValid (Variables|Default|GetNearestEnemy)
            (:Is%20Valid
              (CallFunction|ChangeNearestEnemy)))))
      (else
        (Utilities|IsValid (Variables|Default|GetNearestEnemy)
          (:Is%20Valid
            (CallFunction|ChangeNearestEnemy)))))))

(event Custom|Init
  (bind _asbp_base_character (CallFunction|GetOwnerCharacter))
  (bind _enemydetector (Variables|/Game/Blueprint/Character/BP_BaseCharacter.BP_BaseCharacter_C|GetEnemyDetector _asbp_base_character))
  (bind _overlappingactors (Collision|GetOverlappingActors _enemydetector "/Game/Blueprint/Character/BP_BaseCharacter.BP_BaseCharacter_C" :!class /Script/Engine.PrimitiveComponent))
  (CallFunction|ClearEnemys)
  (if (> (Utilities|Array|Length _overlappingactors) 0)
    (for _array_element _overlappingactors
      (bind _asbp_base_character_2 (Utilities|Casting|CastToBP_BaseCharacter _array_element))
      (Utilities|IsValid _asbp_base_character_2
        (:Is%20Valid
          (if (Math|Boolean|ANDBoolean (!= _asbp_base_character_2 (CallFunction|GetOwnerCharacter)) (Utilities|Enum|Equal(Enum) (Variables|/Game/Blueprint/Character/BP_BaseCharacter.BP_BaseCharacter_C|GetCamp _asbp_base_character_2) "NewEnumerator1") (not (Default|HasAnyAbilitiesTags _asbp_base_character_2 (GameplayTags|MakeLiteralGameplayTagContainer "(GameplayTags=((TagName=\"Combat.Abilities.Lying\"),(TagName=\"Combat.Abilities.Dying\")))") true)))
            (Utilities|Array|AddUnique (Variables|Default|GetPredetectEnemys) _asbp_base_character_2)
            (EventDispatchers|BindEventtoOnTagsChanged _asbp_base_character_2 (delegate Custom|OnTagsChanged))))))))

(event Custom|OnTagsChanged
  (params (Character :type BP%20Base%20Character%20Object%20Reference))
  (bind _predetectenemys (Variables|Default|GetPredetectEnemys))
  (bind _insectorenemy (Variables|Default|GetInSectorEnemy))
  (if (Default|HasAnyAbilitiesTags Character (GameplayTags|MakeLiteralGameplayTagContainer "(GameplayTags=((TagName=\"Combat.Abilities.Lying\"),(TagName=\"Combat.Abilities.Dying\")))") true)
    (Utilities|FlowControl|Sequence
      (:then_0
        (if (Utilities|Array|ContainsItem _predetectenemys Character)
          (Utilities|Array|RemoveItem _predetectenemys Character)))
      (:then_1
        (if (Utilities|Array|ContainsItem _insectorenemy Character)
          (Utilities|Array|RemoveItem _insectorenemy Character)))
      (:then_2
        (CallFunction|TryLockonTarget)))))

(fn GetDisBetweenTargettoOwner
  (params (Target :type BP%20Base%20Character%20Object%20Reference))
  (bind _asbp_base_character (CallFunction|GetOwnerCharacter))
  (bind _returnvalue (Transformation|GetActorLocation Target))
  (bind _returnvalue_2 (Transformation|GetActorLocation _asbp_base_character))
  (bind _returnvalue_3 (- _returnvalue _returnvalue_2))
  (return (Math|Vector2D|Vector2DLength (Math|Vector2D|MakeVector2D (.x _returnvalue_3) (.y _returnvalue_3)))))

(fn IsinSectorArea
  (params (SectorDirection :type Vector) (Angle :type Float%20%28double-precision%29) (TargetCharcter :type BP%20Base%20Character%20Object%20Reference))
  (bind _asbp_base_character (CallFunction|GetOwnerCharacter))
  (bind _returnvalue (Transformation|GetActorLocation TargetCharcter))
  (bind _returnvalue_2 (Transformation|GetActorLocation _asbp_base_character))
  (bind _returnvalue_3 (- _returnvalue _returnvalue_2))
  (return (> (Math|Vector|DotProduct SectorDirection (Math|Vector|Normalize (Math|Vector|MakeVector (.x _returnvalue_3) (.y _returnvalue_3) 0.0))) (- 1.0 (/ Angle 1.8e+02)))))

(fn ChangeNearestEnemy
  (params (NearestEnemy :type BP%20Base%20Character%20Object%20Reference))
  (Utilities|IsValid NearestEnemy
    (:Is%20Valid
      (if (!= NearestEnemy (Variables|Default|GetNearestEnemy))
        (Utilities|IsValid (Variables|Default|GetNearestEnemy)
          (:Is%20Valid
            (Default|ChangeBeenTargetedState (Variables|Default|GetNearestEnemy) false))
          (:Is%20Not%20Valid
            _))
        (bind _output_get (Variables|Default|SetNearestEnemy NearestEnemy))
        (Default|ChangeBeenTargetedState _output_get true)))
    (:Is%20Not%20Valid
      (Utilities|IsValid (Variables|Default|GetNearestEnemy)
        (:Is%20Valid
          (Default|ChangeBeenTargetedState (Variables|Default|GetNearestEnemy) false)
          (Variables|Default|SetNearestEnemy 0))))))