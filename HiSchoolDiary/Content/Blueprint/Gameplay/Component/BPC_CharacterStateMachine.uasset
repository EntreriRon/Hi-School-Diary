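; Character component that runs a data-table-driven state machine, split by network role.
; Clients and the server player build state objects from StatusTable and run their Enter, Update, Exit and Refresh; authority for other controlled characters only records the status enum.
; TriggerTransition, marked server-only, matches the current status and an action against TransitionGraph rows, then calls ChangeState with the next state.
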(event Custom|ChangeState
  (params (NewStatus :type E_CharacterState%20Enum :default "NewEnumerator0"))
  (bind _statusobjs (Variables|ClientData|GetStatusObjs))
  (bind _value (Utilities|Map|Find _statusobjs NewStatus))
  (Utilities|ServerorClient
    (:Authority
      (Variables|ServerOnly|SetCurrentStatus NewStatus))
    (:Remote
      (if (!= (Variables|ClientData|GetCurrStateObj) _value) :!label _label
        (Utilities|IsValid (Variables|ClientData|GetCurrStateObj)
          (:Is%20Valid
            (Default|Exit (Variables|ClientData|GetCurrStateObj)))
          (:Is%20Not%20Valid
            _))
        (Variables|ClientData|SetCurrStateObj _value)
        (Default|Enter (Variables|ClientData|GetCurrStateObj) (CallFunction|GetOwnerCharacter))
        (Development|PrintString (Utilities|String|Append "NewState>>" (Utilities|GetDisplayName _value)))
        (else
          (Default|Refresh (Variables|ClientData|GetCurrStateObj)))))
    (:ServerPlayer
      (Variables|ServerOnly|SetCurrentStatus NewStatus)
      (goto _label))))

(event Custom|TriggerTransition
  (params (TransitionValue :type Gameplay%20Tag%20Structure))
  ;[1 0.364 0.3541] ServerOnly  ---  Automatically transition state to state
  (Variables|ServerOnly|SetFound false)
  ;;[1 1 1] Get current state transition rule
  (bind _rows (CallFunction|GetCurrStateRow))
  (if (> (Utilities|Array|Length _rows) 0)
    (bind _array_element (Utilities|Array|ForEachLoopwithBreak _rows :!label _label)
      (:LoopBody
        (bind _returnvalue (Utilities|GetDataTableRow (Variables|Public|GetTransitionGraph) _array_element)
          (:then
            ;;[1 1 1] ApplyChangeWithMatchTransition
            (if (== (.Action (Utilities|Struct|BreakStruc_CharStateTransition _returnvalue)) TransitionValue)
              (Variables|ServerOnly|SetNextStatus (.NextState (Utilities|Struct|BreakStruc_CharStateTransition _returnvalue)))
              (Variables|ServerOnly|SetFound true)
              (goto _label Break)))))
      (:Completed
        (if (Variables|ServerOnly|GetFound)
          ;;[1 1 1] ChangeState
          (CallFunction|ChangeState (Variables|ServerOnly|GetNextStatus)))))))

(event Custom|ResetStatus
  (CallFunction|ChangeState "NewEnumerator0"))

(event EventTick
  (params (DeltaSeconds :type Float%20%28single-precision%29))
  (Utilities|ServerorClient
    (:Remote
      _)
    (:ServerPlayer
      _))
  (Default|Update (Variables|ClientData|GetCurrStateObj)))

(event EventBeginPlay
  (bind _statustable (Variables|Public|GetStatusTable))
  (Utilities|ServerorClient
    (:Authority
      (Variables|ServerOnly|SetCurrentStatus "NewEnumerator0"))
    (:Remote
      (bind _outrownames (DataTable|GetDataTableRowNames _statustable :!label _label))
      (for _array_element _outrownames
        (bind _returnvalue (Utilities|GetDataTableRow _statustable _array_element)
          (:then
            (if (Utilities|IsValidClass (.StatusObjClass (Utilities|Struct|BreakStuc_CharStatusInfo _returnvalue)))
              (bind _returnvalue_2 (Game|ConstructObjectfromClass (.StatusObjClass (Utilities|Struct|BreakStuc_CharStatusInfo _returnvalue))))
              (bind _output_get (Variables|/Game/Blueprint/Gameplay/CharacterState/CharState_Base.CharState_Base_C|SetState _returnvalue_2 (.Status (Utilities|Struct|BreakStuc_CharStatusInfo _returnvalue))))
              (Utilities|Map|Add (Variables|ClientData|GetStatusObjs) _output_get _returnvalue_2)))))
      (CallFunction|ChangeState "NewEnumerator0"))
    (:ServerPlayer
      (Variables|ServerOnly|SetCurrentStatus "NewEnumerator0")
      (goto _label))))

(fn GetCurrStateRow
  (bind _transitiongraph (Variables|Public|GetTransitionGraph))
  (bind _outrownames (DataTable|GetDataTableRowNames _transitiongraph))
  (for _array_element _outrownames
    (bind _returnvalue (Utilities|GetDataTableRow _transitiongraph _array_element)
      (:then
        (if (Utilities|Array|ContainsItem (Utilities|Struct|BreakStruc_CharStateTransition _returnvalue) (Variables|ServerOnly|GetCurrentStatus))
          (Utilities|Array|Add (LocalVariables|GetLRows) _array_element)))))
  (return (LocalVariables|GetLRows)))

(fn IsCurrentState
  (params (State :type E_CharacterState%20Enum :default "NewEnumerator0"))
  (return (Utilities|Enum|Equal(Enum) (Variables|/Game/Blueprint/Gameplay/CharacterState/CharState_Base.CharState_Base_C|GetState (Variables|ClientData|GetCurrStateObj)) State)))