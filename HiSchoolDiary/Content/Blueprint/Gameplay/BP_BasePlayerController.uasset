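; Base player controller that turns touch, keyboard and gamepad input into character actions.
; Tick prefers the HUD joystick over input axes, moves the character and sets control rotation from the camera-relative direction.
; Keys and gamepad buttons simulate HUD button presses, while action events forward to the character, with Grab choosing throw, pickup, grapple or grab.
; It also shows a network indicator and client info text, and restores travel HP on possession.
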(event Custom|Dash
  (Default|ActionDash (CallFunction|GetControlledCharacter)))

(event Custom|ComboAttack
  (params (Action :type Input%20Action%20Object%20Reference))
  (Default|ActionAttack (CallFunction|GetControlledCharacter)))

(event Custom|SetSprintActive
  (params (Active :type Boolean))
  (Default|ActionSprint (CallFunction|GetControlledCharacter) Active))

(event Custom|AddMovement
  (params (MoveDirection :type Vector%202D%20Structure) (MoveScale :type Float%20%28single-precision%29))
  (Default|ActionMove (CallFunction|GetControlledCharacter) MoveDirection MoveScale)
  (Pawn|SetControlRotation (CallFunction|TransformDesiredMoveRotation MoveDirection)))

(event Custom|ShowInfoText
  (params (text :type String) (time :type Float%20%28double-precision%29))
  ;[1 1 1] exec on owning client
  (Default|ShowInfoText (CallFunction|GetPlayerBaseHUD self) text time))

(event Custom|Grab
  (bind _asbp_base_player (CallFunction|GetControlledCharacter))
  (bind _asbp_base_player_2 (CallFunction|GetControlledCharacter))
  (if (.Equiped (Default|IsEquipedwithWeapon _asbp_base_player_2))
    (Default|ThrowWeapon _asbp_base_player_2)
    (elif (> (Utilities|Array|Length (Variables|/Game/Blueprint/Character/BP_BaseCharacter.BP_BaseCharacter_C|GetPropsAround _asbp_base_player_2)) 0)
      (CallFunction|PickupWeapon)
      (elif (Default|HasAnyAbilitiesTags _asbp_base_player (GameplayTags|MakeLiteralGameplayTagContainer "(GameplayTags=((TagName=\"Combat.Abilities.Grapple\")))") true)
        (Default|TryThrow (Variables|/Game/Blueprint/Character/BP_BaseCharacter.BP_BaseCharacter_C|GetGrappleComponent _asbp_base_player))
        (else
          (Default|ActionGrab _asbp_base_player))))))

(event Custom|PickupWeapon
  (Default|ActionPickupNearestWeapon (CallFunction|GetControlledCharacter)))

(event EventPossess
  (params (PossessedPawn :type Pawn%20Object%20Reference))
  (CallFunction|LoadTravelState))

(event EventBeginPlay
  (Input|SetInputModeGameandUI self 0 "DoNotLock" true)
  (bind _asbp_ui_network (Utilities|Casting|CastToBP_UI_Network (UserInterface|GetWidget (Variables|Default|GetNetworkIndicator))))
  (UserInterface|Viewport|AddtoViewport _asbp_ui_network 0)
  (Default|UpdateIconState _asbp_ui_network))

(event EventTick
  (params (DeltaSeconds :type Float%20%28single-precision%29))
  (bind _basehud (CallFunction|GetPlayerBaseHUD))
  (bind _returnvalue (Class|Actor|GetInputAxisKeyValue))
  (bind _returnvalue_2 (Class|Actor|GetInputAxisKeyValue))
  (bind _returnvalue_3 (Input|AxisValues|GetMoveForward/Backward))
  (bind _returnvalue_4 (Input|AxisValues|GetMoveRight/Left))
  (bind _returnvalue_5 (+ _returnvalue_3 _returnvalue))
  (bind _returnvalue_6 (+ _returnvalue_4 _returnvalue_2))
  (bind _bp_ui_joysitck (Variables|/Game/Blueprint/UI/BP_UI_BaseHUD.BP_UI_BaseHUD_C|GetBP_UI_Joysitck _basehud))
  (bind _returnvalue_7 (Math|Vector2D|MakeVector2D _returnvalue_5 _returnvalue_6))
  (bind _returnvalue_8 (Math|Vector2D|Vector2DLength _returnvalue_7))
  (Utilities|IsValid _basehud
    (:Is%20Valid
      (Utilities|IsValid _bp_ui_joysitck
        (:Is%20Valid
          (if (Variables|/Game/Blueprint/UI/BP_UI_Joystick.BP_UI_Joystick_C|GetisJoystickMoving _bp_ui_joysitck)
            (Variables|Default|SetMove%20Direction (Variables|/Game/Blueprint/UI/BP_UI_Joystick.BP_UI_Joystick_C|GetMoveDirection _bp_ui_joysitck))
            (Variables|Default|SetMove%20Scale (Variables|/Game/Blueprint/UI/BP_UI_Joystick.BP_UI_Joystick_C|GetMoveScale _bp_ui_joysitck))
            (CallFunction|AddMovement (Variables|Default|GetMove%20Direction) (Variables|Default|GetMove%20Scale) :!label _label)
            (else
              (if (> _returnvalue_8 0.0) :!label _label_2
                (Variables|Default|SetMove%20Direction (Math|Vector2D|Normalize2D _returnvalue_7))
                (Variables|Default|SetMove%20Scale (Math|Float|Clamp(Float) _returnvalue_8))
                (goto _label)
                (else
                  (Variables|Default|SetMove%20Scale 0.0))))))
        (:Is%20Not%20Valid
          (goto _label_2))))))

(event Input|ActionEvents|InputActionLightAttack
  (params (Key :type Key%20Structure :default "None"))
  (bind _basehud (CallFunction|GetPlayerBaseHUD))
  (bind _btn_lightatk (Variables|/Game/Blueprint/UI/BP_UI_BaseHUD.BP_UI_BaseHUD_C|GetBtn_LightAtk _basehud))
  ;[1 1 1] Simulate Input Mapping
  (:Pressed
    (Default|OnPress _btn_lightatk))
  (:Released
    (Default|OnRelease _btn_lightatk)))

(event Input|ActionEvents|InputActionHeavyAttack
  (params (Key :type Key%20Structure :default "None"))
  (bind _basehud (CallFunction|GetPlayerBaseHUD))
  (bind _btn_heavyatk (Variables|/Game/Blueprint/UI/BP_UI_BaseHUD.BP_UI_BaseHUD_C|GetBtn_HeavyAtk _basehud))
  ;[1 1 1] Simulate Input Mapping
  (:Pressed
    (Default|OnPress _btn_heavyatk))
  (:Released
    (Default|OnRelease _btn_heavyatk)))

(event Input|ActionEvents|InputActionDash
  (params (Key :type Key%20Structure :default "None"))
  (bind _basehud (CallFunction|GetPlayerBaseHUD))
  (bind _btn_dash (Variables|/Game/Blueprint/UI/BP_UI_BaseHUD.BP_UI_BaseHUD_C|GetBtn_Dash _basehud))
  ;[1 1 1] Simulate Input Mapping
  (:Pressed
    (Default|OnPress _btn_dash))
  (:Released
    (Default|OnRelease _btn_dash)))

(event Input|ActionEvents|InputActionGMPanel
  (params (Key :type Key%20Structure :default "None"))
  (bind _basehud (CallFunction|GetPlayerBaseHUD))
  (:Pressed
    (Utilities|FlowControl|FlipFlop
      (:A
        (Default|ShowGMPanel _basehud true))
      (:B
        (Default|ShowGMPanel _basehud false)))))

(event Input|GamepadEvents|GamepadFaceButtonLeft
  (params (Key :type Key%20Structure :default "None"))
  (bind _basehud (CallFunction|GetPlayerBaseHUD))
  (bind _btn_lightatk (Variables|/Game/Blueprint/UI/BP_UI_BaseHUD.BP_UI_BaseHUD_C|GetBtn_LightAtk _basehud))
  ;[1 1 1] Simulate Input Mapping
  (:Pressed
    (Default|OnPress _btn_lightatk))
  (:Released
    (Default|OnRelease _btn_lightatk)))

(event Input|GamepadEvents|GamepadFaceButtonTop
  (params (Key :type Key%20Structure :default "None"))
  (bind _basehud (CallFunction|GetPlayerBaseHUD))
  (bind _btn_heavyatk (Variables|/Game/Blueprint/UI/BP_UI_BaseHUD.BP_UI_BaseHUD_C|GetBtn_HeavyAtk _basehud))
  ;[1 1 1] Simulate Input Mapping
  (:Pressed
    (Default|OnPress _btn_heavyatk))
  (:Released
    (Default|OnRelease _btn_heavyatk)))

(event Input|GamepadEvents|GamepadFaceButtonBottom
  (params (Key :type Key%20Structure :default "None"))
  (bind _basehud (CallFunction|GetPlayerBaseHUD))
  (bind _btn_dash (Variables|/Game/Blueprint/UI/BP_UI_BaseHUD.BP_UI_BaseHUD_C|GetBtn_Dash _basehud))
  ;[1 1 1] Simulate Input Mapping
  (:Pressed
    (Default|OnPress _btn_dash))
  (:Released
    (Default|OnRelease _btn_dash)))

(event Input|GamepadEvents|GamepadFaceButtonRight
  (params (Key :type Key%20Structure :default "None"))
  ;[1 1 1] Simulate Input Mapping
  (:Pressed
    (Default|OnPress (Variables|/Game/Blueprint/UI/BP_UI_BaseHUD.BP_UI_BaseHUD_C|GetBtn_Grab (CallFunction|GetPlayerBaseHUD)))))

(fn ConstructionScript)

(fn TransformDesiredMoveRotation
  (params (InVec :type Vector%202D%20Structure))
  (bind (_x _y) (Math|Vector2D|BreakVector2D InVec))
  (bind _returnvalue (Game|GetPlayerCameraManager 0))
  (bind _returnvalue_2 (Camera|GetCameraRotation _returnvalue))
  (bind _returnvalue_3 (Math|Vector|MakeVector _x _y 0.0))
  (bind _returnvalue_4 (Class|KismetMathLibrary|NegateRotator _returnvalue_2))
  (bind (_x_2 _y_2) (Math|Rotator|GetAxes _returnvalue_4))
  (return (Math|Conversions|RotationFromXVector (Math|Vector|MakeVector (Math|Vector|DotProduct _x_2 _returnvalue_3) (Math|Vector|DotProduct _y_2 _returnvalue_3) 0.0))))

(fn LoadTravelState
  (bind _returnvalue (Pawn|GetControlledPawn))
  (bind _asbp_hsd_game_state (Utilities|Casting|CastToBP_HSD_GameState (Game|GetGameState)))
  (bind (_travel_data _found) (Default|GetPlayerTravelData _asbp_hsd_game_state (PlayerState|GetUniqueID (Variables|Default|GetPlayerState))))
  (if _found
    (bind _structout (Utilities|Struct|SetmembersinST_PlayerTravelData _travel_data true))
    (if (Utilities|IsValid _returnvalue)
      (bind _asbp_base_player (Utilities|Casting|CastToBP_BasePlayer _returnvalue))
      (Variables|/Game/Blueprint/Character/BP_BaseCharacter.BP_BaseCharacter_C|SetCurrentHP _asbp_base_player (.hp _structout))
      (else
        (Development|PrintString "----- PCtrl::LoadTravelData, error no pawn")))))

(fn FixRot
  (Pawn|SetControlRotation (CallFunction|TransformDesiredMoveRotation (Variables|Default|GetMove%20Direction))))